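; Terrain tile for an infinite-terrain mode that fills itself on BeginPlay with props, rocks and AI characters through PlaceActors and PlaceAIPawns.
; The player entering LockingVolume opens the barrier (green, no collision) and reports the tile conquered once to the InfinateTerrain game mode; leaving relocks it red.
; Reaching DestroyVolume has the game mode spawn another tile and destroys this one.
; An Arrow component supplies the tile's attach transform.
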(event OnComponentBeginOverlap(LockingVolume)
  (params (OverlappedComponent :type Primitive%20Component%20Object%20Reference) (OtherActor :type Actor%20Object%20Reference) (OtherComp :type Primitive%20Component%20Object%20Reference) (OtherBodyIndex :type Integer) (bFromSweep :type Boolean) (SweepResult :type Hit%20Result%20Structure%20%28by%20ref%29))
  (Utilities|IsPlayerActor OtherActor)
  (Utilities|FlowControl|Sequence
    (:then_0
      (CallFunction|Unlock)
      (Utilities|Casting|CastToInfinateTerrain (Game|GetGameMode)))
    (:then_1
      (CallFunction|TileConquered))))

(event OnComponentEndOverlap(LockingVolume)
  (params (OverlappedComponent :type Primitive%20Component%20Object%20Reference) (OtherActor :type Actor%20Object%20Reference) (OtherComp :type Primitive%20Component%20Object%20Reference) (OtherBodyIndex :type Integer))
  (Utilities|IsPlayerActor OtherActor)
  (CallFunction|Lock))

(event OnComponentBeginOverlap(DestroyVolume)
  (params (OverlappedComponent :type Primitive%20Component%20Object%20Reference) (OtherActor :type Actor%20Object%20Reference) (OtherComp :type Primitive%20Component%20Object%20Reference) (OtherBodyIndex :type Integer) (bFromSweep :type Boolean) (SweepResult :type Hit%20Result%20Structure%20%28by%20ref%29))
  (Utilities|IsPlayerActor OtherActor)
  (bind _asinfinate_terrain (Utilities|Casting|CastToInfinateTerrain (Game|GetGameMode)))
  (Default|SpawnTile _asinfinate_terrain)
  (Actor|DestroyActor))

(event EventBeginPlay
  (CallFunction|Lock)
  (Class|Tile|PlaceActors "/Game/Terrain/Props/BP_Container.BP_Container_C" 1 4 4e+02 1.0 1.0)
  (Class|Tile|PlaceActors "/Game/Terrain/Props/BP_Box.BP_Box_C" 0 5 1e+02 1.0 1.0)
  (Class|Tile|PlaceActors "/Game/Terrain/Props/BP_Canister.BP_Canister_C" 0 7 5e+01 1.0 1.0)
  (Class|Tile|PlaceActors "/Game/Terrain/Props/BP_Rock_01.BP_Rock_01_C" 0 3 1.5e+02 1.0 4.0)
  (Class|Tile|PlaceActors "/Game/Terrain/Props/BP_Rock_02.BP_Rock_02_C" 0 3 2.5e+02 1.0 4.0)
  (Class|Tile|PlaceActors "/Game/Terrain/Props/BP_Rock_03.BP_Rock_03_C" 0 3 2.5e+02 1.0 4.0)
  (Class|Tile|PlaceAIPawns "/Game/ThirdPerson/Character_BP.Character_BP_C" 2 4 5e+01))

(event Collision|EventActorBeginOverlap
  (params (OtherActor :type Actor%20Object%20Reference)))

(event EventTick
  (params (DeltaSeconds :type Float%20%28single-precision%29)))

(fn ConstructionScript)

(fn GetAttachLocation
  (return (Transformation|GetWorldTransform (Variables|Default|GetArrow))))

(fn Unlock
  (bind _barrier (Variables|Default|GetBarrier))
  (Collision|SetCollisionEnabled _barrier "NoCollision")
  (Rendering|Material|SetMaterial _barrier 0 "/Game/Geometry/Meshes/GreenBarrier.GreenBarrier"))

(fn Lock
  (bind _barrier (Variables|Default|GetBarrier))
  (Collision|SetCollisionEnabled _barrier "QueryAndPhysics")
  (Rendering|Material|SetMaterial _barrier 0 "/Game/Geometry/Meshes/RedBarrier.RedBarrier"))

(fn TileConquered
  (if (Variables|Default|Getistileconq)
    (return)
    (else
      (bind _asinfinate_terrain (Utilities|Casting|CastToInfinateTerrain (Game|GetGameMode)))
      (Default|NewTileConquered _asinfinate_terrain)
      (Variables|Default|Setistileconq true)
      (return))))