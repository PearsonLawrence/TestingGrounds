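; AI controller for guard NPCs that patrol and track perceived targets.
; On BeginPlay, FindPatrolRoute initializes the PatrolData blackboard and runs the GuardBehavior tree.
; Perception updates set or clear the blackboard enemy key for actors not tagged "Enemy".
; A separate, similarly named "Find Patrol Route" picks a random WayPoint from the pawn's patrol points but is not called here; AimAndShoot is an empty stub.
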(event OnTargetPerceptionUpdated(AIPerception)
  (params (Actor :type Actor%20Object%20Reference) (Stimulus :type AI%20Stimulus%20Structure))
  (CallFunction|UpdateBlackboardEnemyKey Actor Stimulus Actor))

(event EventBeginPlay
  (CallFunction|FindPatrolRoute))

(fn ConstructionScript)

(fn FindPatrolRoute
  (params (BlackBoard :type Blackboard%20Component%20Object%20Reference))
  (bind _asthird_person_character (Utilities|Casting|CastToThirdPersonCharacter (Pawn|GetControlledPawn)))
  (AI|Components|Blackboard|SetValueasObject BlackBoard (Utilities|Name|MakeLiteralName "WayPoint") (Utilities|Array|Get(acopy) (Variables|/Game/ThirdPersonCPP/Blueprints/ThirdPersonCharacter.ThirdPersonCharacter_C|GetPatrol%20Points _asthird_person_character) (Math|Random|RandomInteger 4))))

(fn FindPatrolRoute
  (bind _blackboardcomponent (Class|AIController|UseBlackboard "/Game/AI/PatrolData.PatrolData"))
  (AI|RunBehaviorTree "/Game/AI/GuardBehavior.GuardBehavior")
  (Variables|Default|SetBlackboardcomp _blackboardcomponent))

(fn AimandShoot)

(fn UpdateBlackboardEnemyKey
  (params (ObjectValue :type Object%20Object%20Reference) (AIStimulus :type AI%20Stimulus%20Structure%20%28by%20ref%29) (self2 :type Actor%20Object%20Reference))
  (bind _enemykey (Variables|Default|GetEnemyKey))
  (bind _blackboardcomp (Variables|Default|GetBlackboardcomp))
  (if (not (Actor|ActorHasTag self2 "Enemy"))
    (if (.bSuccessfullySensed (Utilities|Struct|BreakAIStimulus AIStimulus))
      (AI|Components|Blackboard|SetValueasObject _blackboardcomp _enemykey ObjectValue)
      (else
        (AI|Components|Blackboard|ClearValue _blackboardcomp _enemykey)))))